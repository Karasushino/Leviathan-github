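; Player character that aims, throws and recalls a Leviathan axe held as a child actor.
; Holding right mouse sets the aiming state on the Gideon AnimBP and drives a timeline that lerps the camera, reversing at a slower rate on release.
; Left mouse and R play guarded montages: the throw fires on the montage's notify end, while recall triggers on the axe as soon as its montage starts.
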(event EventBeginPlay
  (|CallParentFunction)
  (bind _asgideon_anim_bp (Utilities|Casting|CastToGideon_AnimBP (Components|SkeletalMesh|GetAnimInstance (Variables|Character|GetMesh))))
  (Variables|Default|SetAnim_BP_Ref _asgideon_anim_bp)
  (bind _asleviathan_axe_bp (Utilities|Casting|CastToLeviathanAxe_BP (Variables|/Script/Engine.ChildActorComponent|GetChildActor (Variables|Default|GetLeviathanAxeChildActorComponent))))
  (Variables|Default|SetAxe%20Ref _asleviathan_axe_bp))

(event Input|MouseEvents|LeftMouseButton
  (params (Key :type Key%20Structure :default "None"))
  (:Pressed
    (if (Class|LeviathanCharacter|CanThrowAxe)
      (Animation|Montage|PlayMontage (Variables|Character|GetMesh) "/Game/Character/Animation/Axe/M_ThrowAxe.M_ThrowAxe"
        (:OnNotifyEnd
          (Default|ThrowEvent (Variables|Default|GetAxe%20Ref)))))))

(event Input|KeyboardEvents|R
  (params (Key :type Key%20Structure :default "None"))
  (:Pressed
    (if (Class|LeviathanCharacter|CanRecallAxe)
      (Animation|Montage|PlayMontage (Variables|Character|GetMesh) "/Game/Character/Animation/Axe/RecallAxe_Montage.RecallAxe_Montage"
        (:then
          (Default|RecallEvent (Variables|Default|GetAxe%20Ref)))))))

(event Input|MouseEvents|RightMouseButton
  (params (Key :type Key%20Structure :default "None"))
  (bind _axeaimtimeline (Variables|Default|GetAxeAimTimeline))
  (bind _anim_bp_ref (Variables|Default|GetAnim_BP_Ref))
  (:Pressed
    (bind _output_get (Variables|Default|SetbAiming true))
    (Variables|/Game/Character/Gideon_AnimBP.Gideon_AnimBP_C|SetRangedAttackMode _anim_bp_ref _output_get)
    (Class|LeviathanCharacter|Aim :!label _label)
    (if (Variables|Default|GetbAiming)
      (Components|Timeline|SetPlayRate _axeaimtimeline 1.7)
      (bind _lerpcurve (Timeline|AxeAimTimeline Play)
        (:Update
          (Class|LeviathanCharacter|LerpCameraPosition _lerpcurve)))
      (else
        (Components|Timeline|SetPlayRate _axeaimtimeline 1.2)
        (Timeline|AxeAimTimeline Reverse))))
  (:Released
    (Variables|Default|SetbAiming false)
    (Variables|/Game/Character/Gideon_AnimBP.Gideon_AnimBP_C|SetRangedAttackMode _anim_bp_ref false)
    (goto _label)))

(fn ConstructionScript)